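; LinkedTrap_Rotating is a linked trap in BiomeA that kills the player on overlap while it is active.
; On BeginPlay its non-looping paper flipbook is stopped at the first frame.
; When LinkReaction fires, the trap deactivates and plays the flipbook forward, then after a configurable delay plays it in reverse and immediately reactivates.
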(event EventBeginPlay
  (bind _paperflipbook (Variables|Default|GetPaperFlipbook))
  (|CallParentFunction)
  (Components|Timeline|SetLooping _paperflipbook false)
  (Class|PaperFlipbookComponent|SetPlaybackPositioninFrames _paperflipbook 0 false)
  (Audio|Components|Audio|Stop _paperflipbook))

(event Collision|EventActorBeginOverlap
  (params (OtherActor :type Actor%20Object%20Reference))
  (|CallParentFunction OtherActor)
  (if (Variables|Default|Getactive)
    (bind _aspaper_character_player (Utilities|Casting|CastToPaperCharacter_Player OtherActor))
    (Default|DeathPlayer _aspaper_character_player)))

(event EventLinkReaction
  (bind _paperflipbook (Variables|Default|GetPaperFlipbook))
  (Variables|Default|Setactive false)
  (Components|Timeline|PlayfromStart _paperflipbook)
  (Utilities|FlowControl|Delay (Variables|Default|Getdelay))
  (Components|Timeline|ReversefromEnd _paperflipbook)
  (Variables|Default|Setactive true))

(fn ConstructionScript
  (|CallParentFunction))