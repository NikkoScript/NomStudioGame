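; Ladder actor for the 2D Paper player character, letting the player attach and detach with the Use input.
; Overlap binds or unbinds the player's Use event, which toggles between Attache and Detache; leaving the overlap while attached also detaches.
; Attaching changes the player's state and disables the Actor_Lader_Reception platform's collision.
; Detaching resets the state, restores walking movement and re-enables that collision.
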(event Custom|Use
  (Development|PrintString "Use echelle")
  (if (Variables|Default|Getis_use)
    (CallFunction|Detache)
    (else
      (CallFunction|Attache))))

(event Collision|EventActorBeginOverlap
  (params (OtherActor :type Actor%20Object%20Reference))
  (bind _aspaper_character_player (Utilities|Casting|CastToPaperCharacter_Player OtherActor))
  (EventDispatchers|BindEventtoUse _aspaper_character_player (delegate Custom|Use)))

(event Collision|EventActorEndOverlap
  (params (OtherActor :type Actor%20Object%20Reference))
  (bind _aspaper_character_player (Utilities|Casting|CastToPaperCharacter_Player OtherActor))
  (EventDispatchers|UnbindEventfromUse _aspaper_character_player (delegate Custom|Use))
  (if (Variables|Default|Getis_use)
    (CallFunction|Detache)))

(fn ConstructionScript)

(fn Detache
  (Development|PrintString "Detache")
  (Variables|Default|Setis_use false)
  (bind _aspaper_character_player (Utilities|Casting|CastToPaperCharacter_Player (Game|Player|GetPlayerPawn 0)))
  (Variables|/Game/NomStudioGame/Characters/Player/Blueprint/PaperCharacter_Player.PaperCharacter_Player_C|SetStatePlayer _aspaper_character_player "NewEnumerator0")
  (Pawn|Components|CharacterMovement|SetMovementMode (Variables|/Script/Engine.Character|GetCharacterMovement _aspaper_character_player) "MOVE_Walking" 0)
  (CallFunction|CollisionPlateformeReception true))

(fn Attache
  (Development|PrintString "Attache")
  (Variables|Default|Setis_use true)
  (bind _aspaper_character_player (Utilities|Casting|CastToPaperCharacter_Player (Game|Player|GetPlayerPawn 0)))
  (Variables|/Game/NomStudioGame/Characters/Player/Blueprint/PaperCharacter_Player.PaperCharacter_Player_C|SetStatePlayer _aspaper_character_player "NewEnumerator2")
  (CallFunction|CollisionPlateformeReception false))

(fn CollisionPlateformeReception
  (params (Collision :type Boolean))
  (bind _asactor_lader_reception (Utilities|Casting|CastToActor_Lader_Reception))
  (if Collision
    (Collision|SetCollisionEnabled (Variables|/Game/NomStudioGame/Base/BiomeA/Blueprint/lader/Actor_Lader_Reception.Actor_Lader_Reception_C|Getplateforme _asactor_lader_reception) "QueryAndPhysics")
    (else
      (Collision|SetCollisionEnabled (Variables|/Game/NomStudioGame/Base/BiomeA/Blueprint/lader/Actor_Lader_Reception.Actor_Lader_Reception_C|Getplateforme _asactor_lader_reception) "NoCollision"))))