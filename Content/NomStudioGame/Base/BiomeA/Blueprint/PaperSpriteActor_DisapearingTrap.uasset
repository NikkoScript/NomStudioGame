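; Disappearing trap actor for Biome A that plays its flipbook once when hit and resets when the player dies.
; On begin play, Spawn stops the flipbook at its first frame.
; Hit starts the non-looping animation and binds Respawn to the player character's death event.
; Respawn calls Spawn again to restore the trap, then unbinds itself from that event.
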(event Custom|Respawn
  (CallFunction|Spawn)
  (bind _aspaper_character_player (Utilities|Casting|CastToPaperCharacter_Player (Game|Player|GetPlayerPawn 0)))
  (EventDispatchers|UnbindEventfromDeath _aspaper_character_player (delegate Custom|Respawn)))

(event EventBeginPlay
  (CallFunction|Spawn))

(event Collision|EventHit
  (params (MyComp :type Primitive%20Component%20Object%20Reference) (Other :type Actor%20Object%20Reference) (OtherComp :type Primitive%20Component%20Object%20Reference) (bSelfMoved :type Boolean) (HitLocation :type Vector :default "0, 0, 0") (HitNormal :type Vector :default "0, 0, 0") (NormalImpulse :type Vector :default "0, 0, 0") (Hit :type Hit%20Result%20Structure%20%28by%20ref%29))
  (Audio|Components|Audio|Play (Variables|Default|GetPaperFlipbook))
  (Components|Timeline|SetLooping (Variables|Default|GetPaperFlipbook) false)
  (bind _aspaper_character_player (Utilities|Casting|CastToPaperCharacter_Player (Game|Player|GetPlayerPawn 0)))
  (EventDispatchers|BindEventtoDeath _aspaper_character_player (delegate Custom|Respawn)))

(fn ConstructionScript)

(fn Spawn
  (bind _paperflipbook (Variables|Default|GetPaperFlipbook))
  (Class|PaperFlipbookComponent|SetPlaybackPositioninFrames _paperflipbook 0 false)
  (Audio|Components|Audio|Stop _paperflipbook))