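; RotatingTrap is a trap actor that kills the PaperCharactertest player on overlap while its kill zone is active.
; LinkReaction temporarily disarms it, swapping active and inactive visuals around a non-looping transition animation and turning off kill zone collision.
; After the Delaykill delay it re-arms the kill zone and plays the same animation in reverse back to the active visual.
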(event EventBeginPlay
  (|CallParentFunction)
  (Components|Timeline|SetLooping (Variables|Default|Getanim) false))

(event Collision|EventActorBeginOverlap
  (params (OtherActor :type Actor%20Object%20Reference))
  (|CallParentFunction OtherActor)
  (if (Variables|Default|Getkillzoneactiv)
    (bind _aspaper_charactertest (Utilities|Casting|CastToPaperCharactertest OtherActor))
    (Default|Deathplayer _aspaper_charactertest)))

(event EventLinkReaction
  (Rendering|SetVisibility (Variables|Default|Getactivatetrap.) false false)
  (CallFunction|Animation false)
  (Utilities|FlowControl|Delay 1.0)
  (Rendering|SetVisibility (Variables|Default|Getdeactivatetrap) true false)
  (Variables|Default|Setkillzoneactiv false)
  (Collision|SetCollisionEnabled (Variables|Default|GetKillzone) "NoCollision")
  (Utilities|FlowControl|Delay (Variables|Default|Getdelaykill))
  (Variables|Default|Setkillzoneactiv true)
  (Development|PrintString "activation piege")
  (Collision|SetCollisionEnabled (Variables|Default|GetKillzone) "QueryOnly")
  (Rendering|SetVisibility (Variables|Default|Getdeactivatetrap) false false)
  (CallFunction|Animation true)
  (Utilities|FlowControl|Delay 1.0)
  (Rendering|SetVisibility (Variables|Default|Getactivatetrap.) true false))

(fn ConstructionScript
  (|CallParentFunction))

(fn Animation
  (params (reverse :type Boolean))
  (Rendering|SetVisibility (Variables|Default|Getanim) true false)
  (if reverse
    (Components|Timeline|ReversefromEnd (Variables|Default|Getanim))
    (else
      (Components|Timeline|PlayfromStart (Variables|Default|Getanim)))))