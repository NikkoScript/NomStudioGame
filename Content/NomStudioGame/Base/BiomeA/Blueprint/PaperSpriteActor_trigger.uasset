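; Trigger actor with two Paper2D sprites that sets off a linked trap when another actor overlaps it.
; An overlap while active calls the linked trap's LinkReaction, then deactivates the trigger until a configurable timer delay re-arms it.
; Every tick, it toggles visibility between the active and inactive sprites to match its state.
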(event EventBeginPlay)

(event Collision|EventActorBeginOverlap
  (params (OtherActor :type Actor%20Object%20Reference))
  (if (Variables|Default|Getactive)
    (Variables|Default|Setactive false)
    (Default|LinkReaction (Variables|Default|GetLinkedTrap))
    (Utilities|FlowControl|Delay (Variables|Default|Gettimer))
    (Variables|Default|Setactive true)))

(event EventTick
  (params (DeltaSeconds :type Float%20%28single-precision%29))
  (bind _paperspriteactive (Variables|Default|GetPaperSpriteActive))
  (bind _paperspriteinactive (Variables|Default|GetPaperSpriteInactive))
  (if (Variables|Default|Getactive)
    (Rendering|SetVisibility _paperspriteactive true false)
    (Rendering|SetVisibility _paperspriteinactive false false)
    (else
      (Rendering|SetVisibility _paperspriteactive false false)
      (Rendering|SetVisibility _paperspriteinactive true false))))

(fn ConstructionScript)